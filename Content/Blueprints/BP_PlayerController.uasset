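; BP_PlayerController is a player controller that turns cursor clicks into world locations for unit movement and building.
; On BeginPlay it binds one event to both the move-to and build-to dispatchers of BP_Player.
; That event traces under the cursor on the Visibility channel, then sends the hit location and hit flag to every BP_AdventurerUnit and every W_GameUI widget.
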(event Custom|GetCursorLocation
  (bind _hitresult (Game|Player|GetHitResultUnderCursorbyChannel "TraceTypeQuery1" true))
  (bind (_bblockinghit _binitialoverlap _time _distance _location) (Collision|BreakHitResult _hitresult))
  (bind _output_get (Variables|Default|SetIsHit _bblockinghit))
  (bind _output_get_2 (Variables|Default|SetCursorLocation _location))
  (bind _outactors (Actor|GetAllActorsOfClass "/Game/Blueprints/BP_AdventurerUnit.BP_AdventurerUnit_C"))
  (Default|MoveUnitto _outactors _output_get_2 _output_get)
  (bind _foundwidgets (Widget|GetAllWidgetsOfClass "/Game/Widgets/W_GameUI.W_GameUI_C" false))
  (Default|GetMouseCursor _foundwidgets _output_get _output_get_2))

(event EventBeginPlay
  (bind _asbp_player (Utilities|Casting|CastToBP_Player (Game|Player|GetPlayerPawn 0)))
  (EventDispatchers|BindEventtoDispatcherMoveto _asbp_player (delegate Custom|GetCursorLocation))
  (EventDispatchers|BindEventtoDispatcherBuildto _asbp_player (delegate Custom|GetCursorLocation)))

(event EventTick
  (params (DeltaSeconds :type Float%20%28single-precision%29)))

(fn ConstructionScript)