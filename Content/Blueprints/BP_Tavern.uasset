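; Clickable tavern building where the player buys adventurer units with food and gold.
; Clicking shows the selection ring and W_TavernPopup widgets, and BP_Player's deselect dispatcher hides them.
; The popup created at BeginPlay binds its spawn event, while a second, unbound one is created on click.
; Spawning checks both resources, places a BP_AdventurerUnit at a fixed offset, plays a coin sound and deducts the cost.
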(event OnClicked(Collision)
  (params (TouchedComponent :type Primitive%20Component%20Object%20Reference) (ButtonPressed :type Key%20Structure :default "None"))
  (Variables|Default|GetPopupUI
    (:then
      _)
    (:else
      (bind _returnvalue (UserInterface|CreateWidget "/Game/Widgets/W_TavernPopup.W_TavernPopup_C"))
      (bind _output_get (Variables|Default|SetPopupUI _returnvalue))))
  (UserInterface|Viewport|AddtoViewport _output_get 0)
  (Class|PrimitiveComponent|SetVisibleinSceneCaptureOnly (Variables|Default|GetSelect%20Ring) false)
  (Variables|Default|SetIsSelected true))

(event Custom|Deselect
  (if (Variables|Default|GetIsSelected)
    (Widget|RemovefromParent (stale OnClicked(Collision) _output_get))
    (Class|PrimitiveComponent|SetVisibleinSceneCaptureOnly (Variables|Default|GetSelect%20Ring) true)
    (Variables|Default|SetIsSelected false)))

(event Custom|OnButtonPress
  (bind _returnvalue (Transformation|GetActorTransform))
  (bind _location (Math|Transform|BreakTransform _returnvalue))
  (bind (_x _y _z) (Math|Vector|BreakVector _location))
  (if (>= (Variables|/Game/Blueprints/BP_Player.BP_Player_C|GetCurrentFood (stale EventBeginPlay _asbp_player)) 50)
    (if (>= (Variables|/Game/Blueprints/BP_Player.BP_Player_C|GetCurrentGold (stale EventBeginPlay _asbp_player)) 100)
      (Game|SpawnActorfromClass "/Game/Blueprints/BP_AdventurerUnit.BP_AdventurerUnit_C" (Math|Conversions|ToTransform(Vector) (Math|Vector|MakeVector (+ _x 5e+02) _y (+ _z 1e+02))) "AdjustIfPossibleButAlwaysSpawn" "MultiplyWithRoot" 0 0)
      (Audio|PlaySoundatLocation "/Game/Sounds/140382__dwoboyle__coins-01.140382__dwoboyle__coins-01" (Transformation|GetWorldLocation (Variables|Default|GetCollision)) "0, 0, 0" 1.0 1.0 0.0 0 0 0 0)
      (bind _asbp_player (Utilities|Casting|CastToBP_Player (Game|Player|GetPlayerPawn 0)))
      (Default|EditCurrentFood _asbp_player -50)
      (Default|EditCurrentGold _asbp_player -100))))

(event EventBeginPlay
  (Class|PrimitiveComponent|SetVisibleinSceneCaptureOnly (Variables|Default|GetSelect%20Ring) true)
  (bind _returnvalue (UserInterface|CreateWidget "/Game/Widgets/W_TavernPopup.W_TavernPopup_C"))
  (EventDispatchers|BindEventtoSpawnAdventurer _returnvalue (delegate Custom|OnButtonPress))
  (bind _asbp_player (Utilities|Casting|CastToBP_Player (Game|Player|GetPlayerPawn 0)))
  (EventDispatchers|BindEventtoDispatcherDeselect _asbp_player (delegate Custom|Deselect)))

(event Collision|EventActorBeginOverlap
  (params (OtherActor :type Actor%20Object%20Reference)))

(event EventTick
  (params (DeltaSeconds :type Float%20%28single-precision%29)))

(fn ConstructionScript)