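; Selectable combat unit pawn with a Viking mesh that moves to cursor-picked ground points.
; Clicking the capsule selects it and reveals SelectRing, while the player's Deselect dispatcher hides the ring by making it scene-capture-only.
; The player's MoveTo dispatcher sends selected units via AI MoveTo to the controller's cursor hit location and spawns a cursor effect there.
; Mesh yaw interpolates toward velocity once per order, not on Tick.
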(event OnClicked(CapsuleCollision)
  (params (TouchedComponent :type Primitive%20Component%20Object%20Reference) (ButtonPressed :type Key%20Structure))
  (Class|PrimitiveComponent|SetVisibleinSceneCaptureOnly (Variables|Default|GetSelect%20Ring) false)
  (Variables|Default|SetIsSelected true))

(event Custom|Deselect
  (Class|PrimitiveComponent|SetVisibleinSceneCaptureOnly (Variables|Default|GetSelect%20Ring) true)
  (Variables|Default|SetIsSelected false))

(event Custom|MoveTo
  (bind _returnvalue (Transformation|GetVelocity))
  (if (Variables|Default|GetIsSelected)
    (Variables|Default|SetStartLocation (Transformation|GetActorLocation))
    (if (Variables|/Game/Blueprints/BP_PlayerController.BP_PlayerController_C|GetIsHit (stale EventBeginPlay _asbp_player_controller))
      (bind _output_get (Variables|Default|SetMoveToDestination (Variables|/Game/Blueprints/BP_PlayerController.BP_PlayerController_C|GetCursorLocation (stale EventBeginPlay _asbp_player_controller))))
      (AI|AIMoveTo self _output_get 0 1e+02 false
        (:then
          (Niagara|SpawnSystematLocation (Variables|Default|GetFXCursor) _output_get)
          (if (> (Math|Vector|VectorLength _returnvalue) 0.1)
            (Transformation|SetWorldRotation (Variables|Default|GetSK_Viking) (Math|Rotator|MakeRotator 0.0 0.0 (.yaw (Math|Interpolation|RInterpTo (Math|Rotator|MakeRotator 0.0 0.0 (.yaw (Transformation|GetWorldRotation (Variables|Default|GetSK_Viking)))) (Math|Rotator|MakeRotator 0.0 0.0 (.yaw (Math|Rotator|MakeRotfromX _returnvalue))) 0.0 5.0))) true true)))))))

(event EventBeginPlay
  (bind _returnvalue (Transformation|GetActorLocation))
  (Transformation|SetRelativeLocation (Variables|Default|GetCapsule%20Collision) (Math|Vector|MakeVector (.x _returnvalue) (.y _returnvalue) 76.26) false true)
  (Class|PrimitiveComponent|SetVisibleinSceneCaptureOnly (Variables|Default|GetSelect%20Ring) true)
  (bind _asbp_player (Utilities|Casting|CastToBP_Player (Game|Player|GetPlayerPawn 0)))
  (EventDispatchers|BindEventtoDispatcherDeselect _asbp_player (delegate Custom|Deselect))
  (EventDispatchers|BindEventtoDispatcherMoveto _asbp_player (delegate Custom|MoveTo))
  (bind _asbp_player_controller (Utilities|Casting|CastToBP_PlayerController (Game|GetPlayerController 0))))

(event Collision|EventActorBeginOverlap
  (params (OtherActor :type Actor%20Object%20Reference)))

(event EventTick
  (params (DeltaSeconds :type Float%20%28single-precision%29)))

(fn ConstructionScript)