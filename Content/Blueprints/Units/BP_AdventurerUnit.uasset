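; BP_AdventurerUnit is an adventurer unit that is selected by click and moved to a target location.
; Clicking the capsule selects it and shows SelectRing, toggled through scene-capture-only visibility.
; BP_Player's deselect dispatcher, bound on BeginPlay, clears selection and hides the ring.
; MoveUnitTo runs AIMoveTo for selected units given a valid hit, spawning a cursor effect at the destination as the move starts.
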(event OnClicked(CapsuleComponent)
  (params (TouchedComponent :type Primitive%20Component%20Object%20Reference) (ButtonPressed :type Key%20Structure :default "None"))
  (Class|PrimitiveComponent|SetVisibleinSceneCaptureOnly (Variables|Default|GetSelect%20Ring) false)
  (Variables|Default|SetIsSelected true))

(event Custom|Move%20Unit%20To
  (params (Location :type Vector) (Is%20Hit :type Boolean))
  (if Is%20Hit
    (if (Variables|Default|GetIsSelected)
      (bind _output_get (Variables|Default|SetMoveToDestination Location))
      (AI|AIMoveTo self _output_get 0 5e+01 false
        (:then
          (Niagara|SpawnSystematLocation (Variables|Default|GetFXCursor) _output_get))))))

(event Custom|Deselect
  (Class|PrimitiveComponent|SetVisibleinSceneCaptureOnly (Variables|Default|GetSelect%20Ring) true)
  (Variables|Default|SetIsSelected false))

(event EventBeginPlay
  (Class|PrimitiveComponent|SetVisibleinSceneCaptureOnly (Variables|Default|GetSelect%20Ring) true)
  (bind _asbp_player (Utilities|Casting|CastToBP_Player (Game|Player|GetPlayerPawn 0)))
  (EventDispatchers|BindEventtoDispatcherDeselect _asbp_player (delegate Custom|Deselect)))

(fn ConstructionScript)