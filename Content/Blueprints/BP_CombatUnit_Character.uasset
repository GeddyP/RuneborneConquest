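; BP_CombatUnit_Character is a click-selectable combat unit that moves to ordered locations while selected.
; Clicking its capsule sets IsSelected and shows SelectRing, which is otherwise hidden from the main view through the scene-capture-only visibility flag.
; On BeginPlay it binds Deselect to a BP_Player dispatcher, which clears the selection.
; MoveTo runs AIMoveTo for selected units and spawns the FXCursor effect at the destination as the order is issued.
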(event OnClicked(CapsuleComponent)
  (params (TouchedComponent :type Primitive%20Component%20Object%20Reference) (ButtonPressed :type Key%20Structure :default "None"))
  (Class|PrimitiveComponent|SetVisibleinSceneCaptureOnly (Variables|Default|GetSelect%20Ring) false)
  (Variables|Default|SetIsSelected true))

(event Custom|Deselect
  (Class|PrimitiveComponent|SetVisibleinSceneCaptureOnly (Variables|Default|GetSelect%20Ring) true)
  (Variables|Default|SetIsSelected false))

(event Custom|MoveTo
  (params (Location :type Vector) (IsHit :type Boolean))
  (if (Variables|Default|GetIsSelected)
    (bind _output_get (Variables|Default|SetMoveToDestination Location))
    (AI|AIMoveTo self _output_get 0 5e+01 false
      (:then
        (Niagara|SpawnSystematLocation (Variables|Default|GetFXCursor) _output_get)))))

(event EventBeginPlay
  (Class|PrimitiveComponent|SetVisibleinSceneCaptureOnly (Variables|Default|GetSelect%20Ring) true)
  (bind _asbp_player (Utilities|Casting|CastToBP_Player (Game|Player|GetPlayerPawn 0)))
  (EventDispatchers|BindEventtoDispatcherDeselect _asbp_player (delegate Custom|Deselect)))

(fn ConstructionScript)