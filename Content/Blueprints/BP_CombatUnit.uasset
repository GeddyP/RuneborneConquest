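; BP_CombatUnit is a click-selectable unit that moves to the player's cursor location on command.
; Clicking its capsule sets IsSelected and reveals a select ring, while dispatchers on BP_Player trigger Deselect and MoveTo.
; When selected, it reads the hit location from BP_PlayerController and lerps there on a timeline at fixed height, without pathfinding.
; A cursor Niagara effect spawns at the destination on every timeline update.
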(event OnClicked(CapsuleCollision)
  (params (TouchedComponent :type Primitive%20Component%20Object%20Reference) (ButtonPressed :type Key%20Structure :default "None"))
  (Class|PrimitiveComponent|SetVisibleinSceneCaptureOnly (Variables|Default|GetSelect%20Ring) false)
  (Variables|Default|SetIsSelected true))

(event Custom|Deselect
  (Class|PrimitiveComponent|SetVisibleinSceneCaptureOnly (Variables|Default|GetSelect%20Ring) true)
  (Variables|Default|SetIsSelected false))

(event Custom|MoveTo
  (if (Variables|Default|GetIsSelected)
    (Variables|Default|SetStartLocation (Transformation|GetActorLocation))
    (if (Variables|/Game/Blueprints/BP_PlayerController.BP_PlayerController_C|GetIsHit (stale EventBeginPlay _asbp_player_controller))
      (bind _output_get (Variables|Default|SetMoveToDestination (Variables|/Game/Blueprints/BP_PlayerController.BP_PlayerController_C|GetCursorLocation (stale EventBeginPlay _asbp_player_controller))))
      (bind _movement (Timeline|TL_MoveToDestination PlayFromStart)
        (:Update
          (Transformation|SetActorLocationAndRotation (Math|Vector|Lerp(Vector) (Variables|Default|GetStartLocation) (Math|Vector|MakeVector (.x _output_get) (.y _output_get) 76.26) _movement) (Transformation|GetActorRotation) false true)
          (Niagara|SpawnSystematLocation (Variables|Default|GetFXCursor) (Variables|Default|GetMoveToDestination)))))))

(event EventBeginPlay
  (bind _returnvalue (Transformation|GetActorLocation))
  (Transformation|SetRelativeLocation (Variables|Default|GetCapsule%20Collision) (Math|Vector|MakeVector (.x _returnvalue) (.y _returnvalue) 76.26) false true)
  (Class|PrimitiveComponent|SetVisibleinSceneCaptureOnly (Variables|Default|GetSelect%20Ring) true)
  (bind _asbp_player (Utilities|Casting|CastToBP_Player (Game|Player|GetPlayerPawn 0)))
  (EventDispatchers|BindEventtoDispatcherDeselect _asbp_player (delegate Custom|Deselect))
  (EventDispatchers|BindEventtoDispatcherMoveto _asbp_player (delegate Custom|MoveTo))
  (bind _asbp_player_controller (Utilities|Casting|CastToBP_PlayerController (Game|GetPlayerController 0))))

(event Collision|EventActorBeginOverlap
  (params (OtherActor :type Actor%20Object%20Reference)))

(event EventTick
  (params (DeltaSeconds :type Float%20%28single-precision%29)))

(fn ConstructionScript)